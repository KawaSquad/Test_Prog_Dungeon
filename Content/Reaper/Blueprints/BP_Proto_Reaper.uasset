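; Prototype Reaper player character with double jump, energy-costing fireball and a charged air dash.
; Tick handles movement and look, smooths input values and line-traces downward to detect being airborne.
; Holding Dash midair freezes movement, changes Energy and builds dash time; release launches along the camera in zero-gravity flight.
; Timeout, capsule hit or another press ends the dash with an explosion, via OnDashStop or directly; BeginPlay also streams ThroneRoom.
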(event `self.ReceiveTick`
  (params (DeltaSeconds :type "Float (single-precision)"))
  (bind _returnvalue (`GameplayStatics.GetPlayerPawn` 0))
  (bind _returnvalue_2 (`self.K2_GetActorLocation`))
  (bind _returnvalue_3 (`self.GetInputAxisValue`))
  (bind _returnvalue_4 (`self.GetInputAxisValue`))
  (bind _returnvalue_5 (* (`GameplayStatics.GetWorldDeltaSeconds`) (`self.SmoothInput`)))
  ;[1 1 1] Update
  (set `self.Forward` (`KismetMathLibrary.Lerp` (`self.Forward`) _returnvalue_3 _returnvalue_5))
  (bind (_outhit _returnvalue_6) (`KismetSystemLibrary.LineTraceSingle` _returnvalue_2 (+ _returnvalue_2 (0.0 0.0 -250.0)) "TraceTypeQuery1"))
  (set `self.IsInAir` (not _returnvalue_6))
  (if (`self.Charging`)
    (`self.Add_Energy` (* (`GameplayStatics.GetWorldDeltaSeconds`) (`self.ChargingCost`)))
    (`self.Add_DashDelay`)
    (elif (`self.Dashing`)
      (`self.Decrease_Delay`)))
  (if (not (`self.Dashing`))
    (if (not (`self.Charging`))
      (`self.AddMovementInput` (`self.GetActorForwardVector` _returnvalue) _returnvalue_3)
      (set `self.Right` (`KismetMathLibrary.Lerp` (`self.Right`) _returnvalue_4 _returnvalue_5))
      (`self.AddMovementInput` (`self.GetActorRightVector` _returnvalue) _returnvalue_4))
    (`self.AddControllerYawInput` (`self.GetInputAxisValue`))
    (`self.AddControllerPitchInput` (`self.GetInputAxisValue`))))

(event `InputAction|Jump`
  (params (Key :type "Key Structure"))
  (bind _returnvalue (`KismetMathLibrary.MakeVector` 0.0 0.0 (`self.ForceJump`)))
  ;[1 1 1] Jumpping
  (:`Pressed`
    (if (`NavMovementComponent.IsFalling` (`self.CharacterMovement`))
      (if (not (`self.DoubleJump`))
        (`self.LaunchCharacter` (`GameplayStatics.GetPlayerCharacter` 0) _returnvalue false true)
        (set `self.DoubleJump` true)
        (`GameplayStatics.PlaySoundAtLocation` "/Game/Reaper/Audio/woosh.woosh" (`self.K2_GetActorLocation`) (struct) 1.0 1.0 0.0 null null null :!label _label)
        (`self.OnJump`))
      (else
        (`self.LaunchCharacter` _returnvalue false true)
        (set `self.DoubleJump` false)
        (goto _label)))))

(event `InputAction|Fireball` :consume false
  (params (Key :type "Key Structure"))
  (bind _mesh (`self.Mesh`))
  ;[1 1 1] Fireball
  (:`Pressed`
    (if (not (`self.IsThrowing`))
      (set `self.IsThrowing` true)
      (if (>= (`self.Energy`) (`self.FireballCost`))
        (bind _returnvalue (`GameplayStatics.SpawnEmitterAttached` "/Game/Reaper/FX/P_CastFire.P_CastFire" _mesh "R_HandSocket" (0.0 0.0 0.0) (struct) (1.0 1.0 1.0) "KeepRelativeOffset" false))
        (`KismetSystemLibrary.Delay` 0.5)
        (`ActorComponent.K2_DestroyComponent` _returnvalue)
        (`|SpawnActorFromClass` "/Game/Reaper/Blueprints/BP_Fireball.BP_Fireball_C" (`KismetMathLibrary.MakeTransform` (`SceneComponent.GetSocketLocation` _mesh "R_HandSocket") (`SceneComponent.K2_GetComponentRotation` (`self.Camera`)) (.scale (`self.GetTransform`))) "Undefined" "OverrideRootScale" null null)
        (`self.Add_Energy` (* (`self.FireballCost`) -1.0))
        (else
          (bind _returnvalue_2 (`GameplayStatics.SpawnEmitterAttached` "/Game/Reaper/FX/P_CastFail.P_CastFail" (`self.Mesh`) "R_HandSocket" (0.0 0.0 0.0) (struct) (1.0 1.0 1.0) "KeepRelativeOffset" false))
          (`KismetSystemLibrary.Delay` 0.5)
          (`ActorComponent.K2_DestroyComponent` _returnvalue_2)
          (`GameplayStatics.PlaySoundAtLocation` "/Game/Reaper/Audio/EnergyFail.EnergyFail" (`self.K2_GetActorLocation`) (struct) 1.0 1.0 0.0 null null null)))
      (`KismetSystemLibrary.Delay` (`self.DelayFireball`))
      (set `self.IsThrowing` false))))

(event `InputAction|Dash` :consume false
  (params (Key :type "Key Structure"))
  (bind _charactermovement (`self.CharacterMovement`))
  (bind _mesh (`self.Mesh`))
  (bind (_returnvalue_location _returnvalue_rotation) (`KismetMathLibrary.BreakTransform` (`SceneComponent.GetSocketTransform` _mesh "TorsoSocket" "RTS_World")))
  ;[1 1 1] Charging_Dashing
  (:`Pressed`
    (`self.OnDashStop`)
    (if (`self.IsInAir`)
      (if (not (`self.Dashing`))
        (set `self.Charging` true)
        (`CharacterMovementComponent.DisableMovement` _charactermovement)
        (bind _returnvalue (`GameplayStatics.SpawnEmitterAtLocation` "/Game/Reaper/FX/P_Charge.P_Charge" (`self.K2_GetActorLocation`)))
        (set `self.charge_particle` _returnvalue))))
  (:`Released`
    (if (`self.Charging`)
      (set `self.Charging` false)
      (set `self.Dashing` true)
      (`ActorComponent.K2_DestroyComponent` (`self.charge_particle`))
      (`CharacterMovementComponent.SetMovementMode` _charactermovement "MOVE_Flying" 0)
      (set `CharacterMovementComponent.GravityScale` 0.0 _charactermovement)
      (`self.LaunchCharacter` (`GameplayStatics.GetPlayerCharacter` 0) (* (`SceneComponent.GetForwardVector` (`self.Camera`)) (`self.DashForce`)) true true)
      (bind _returnvalue_2 (`GameplayStatics.SpawnEmitterAttached` "/Game/Reaper/FX/P_Dash.P_Dash" _mesh "TorsoSocket" _returnvalue_location _returnvalue_rotation (1.0 1.0 1.0) "KeepWorldPosition" true "AutoRelease"))
      (set `self.dash_particle` _returnvalue_2))))

(event `self.ReceiveBeginPlay`
  ;[1 1 1] Delegate end dash
  (set `self.StartGravity` (`CharacterMovementComponent.GravityScale` (`self.CharacterMovement`)))
  (`self.EnableInput` (`GameplayStatics.GetPlayerController` 0))
  (`GameplayStatics.LoadStreamLevel` "ThroneRoom" true)
  (add `self.OnDashStop` (delegate `CustomEvent`)))

(event `CustomEvent`
  (bind _charactermovement (`self.CharacterMovement`))
  ;[1 1 1] Delegate end dash
  ;[1 1 1] End dash
  (if (`self.Dashing`) :!label _label_2
    (set `self.Dashing` false)
    (`CharacterMovementComponent.SetMovementMode` _charactermovement "MOVE_Walking" 0)
    (`ActorComponent.K2_DestroyComponent` (`self.dash_particle`))
    (set `CharacterMovementComponent.GravityScale` (`self.StartGravity`) _charactermovement)
    (`CharacterMovementComponent.ClearAccumulatedForces` _charactermovement)
    (`GameplayStatics.PlaySoundAtLocation` "/Game/StarterContent/Audio/Explosion_Cue.Explosion_Cue" (`self.K2_GetActorLocation`) (struct) 1.0 1.0 0.0 null null null)
    (`GameplayStatics.SpawnEmitterAtLocation` "/Game/Reaper/FX/P_Explosion.P_Explosion" (`.ImpactPoint` (`GameplayStatics.BreakHitResult` (stale `self.CapsuleComponent.OnComponentHit` Hit))))))

(event `self.CapsuleComponent.OnComponentHit`
  (params (HitComponent :type "PrimitiveComponent Object Reference") (OtherActor :type "Actor Object Reference") (OtherComp :type "PrimitiveComponent Object Reference") (NormalImpulse :type "Vector Structure") (Hit :type "HitResult Structure (by ref)"))
  ;[1 1 1] End dash
  (goto _label_2))

(fn `Add_DashDelay`
  (set `self.DelayDash` (+ (`self.DelayDash`) (* (`GameplayStatics.GetWorldDeltaSeconds`) (`self.ChargingDelay`)))))

(fn `Add_Energy`
  (params (Value :type "Float (double-precision)"))
  (set `self.Energy` (`KismetMathLibrary.FClamp` (+ (`self.Energy`) Value) 0.0 100.0)))

(fn `Add_Heal`
  (params (Value :type "Float (double-precision)"))
  (set `self.Health` (`KismetMathLibrary.FClamp` (+ (`self.Health`) Value) 0.0 100.0)))

(fn `Decrease_Delay`
  (bind _output_get (set `self.DelayDash` (- (`self.DelayDash`) (* (`GameplayStatics.GetWorldDeltaSeconds`) (`self.ChargingDelay`)))))
  (if (<= _output_get 0.0)
    (`self.OnDashStop`)
    (set `self.DelayDash` 0.0)))

(fn `Get_Forward`
  (returns (Forward :type "Float (double-precision)"))
  (return (`self.Forward`)))

(fn `Get_IsInAir`
  (returns (IsInAir :type Boolean))
  (return (`self.IsInAir`)))

(fn `Get_Right`
  (returns (Right :type "Float (double-precision)"))
  (return (`self.Right`)))

(fn `UserConstructionScript`)